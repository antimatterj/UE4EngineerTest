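; BP_Cambot is a self-driving camera pawn that wanders the level and captures screen data as it goes.
; On BeginPlay it is possessed by the first player controller, then loops endlessly: move, wait TravelInterval, call CaptureScreenData.
; Roomba teleports it forward by TravelDistance when CanTravel passes, otherwise calls RotateRandom and syncs the player's control rotation to the new facing.
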(event EventBeginPlay
  (Pawn|Possess (Game|GetPlayerController 0) self)
  (CallFunction|Roomba :!label _label) ; Moves forward if no collision, otherwise rotate.
  (Utilities|FlowControl|Delay (Variables|Default|GettravelInterval))
  (Class|Cambot|CaptureScreenData)
  (goto _label))

(fn ConstructionScript)

(fn Roomba
  (if (Class|Cambot|CanTravel)
    (Transformation|SetActorLocation (+ (Transformation|GetActorLocation) (* (Math|Vector|GetForwardVector (Transformation|GetActorRotation)) (Variables|Default|GettravelDistance))) false true)
    (else
      (Class|Cambot|RotateRandom)
      (if (== (Pawn|GetController) (Game|GetPlayerController 0))
        (Pawn|SetControlRotation (Game|GetPlayerController 0) (Transformation|GetActorRotation))))))