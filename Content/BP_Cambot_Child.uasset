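; BP_Cambot_Child is a self-driving camera bot that roams the level, capturing screen data as it goes.
; On BeginPlay, player controller 0 possesses it and an endless loop starts.
; Each pass calls Roomba, which moves forward or rotates on collision, waits TravelInterval, runs CaptureScreenData, then spawns a capture marker at the bot's transform.
; The construction script only calls the parent's.
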(event EventBeginPlay
  (Pawn|Possess (Game|GetPlayerController 0) self)
  (CallFunction|Roomba :!label _label) ; Moves forward if no collision, otherwise rotate.
  (Utilities|FlowControl|Delay (Variables|Default|GettravelInterval))
  (Class|Cambot|CaptureScreenData)
  (Game|SpawnActorfromClass "/Game/BP_Cambot_Capture_Marker.BP_Cambot_Capture_Marker_C" (Transformation|GetActorTransform) "Undefined" 0 0)
  (goto _label))

(fn ConstructionScript
  (|CallParentFunction))